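; BP_Timeline is a test Blueprint that exercises the controls of a single Timeline node.
; Separate events drive Timeline_0's Play, PlayFromStart, Stop, Reverse, ReverseFromEnd and SetNewTime inputs.
; Each update prints the playback direction joined with the values of two tracks, and completion prints a finished message.
; BeginPlay, Tick, overlap and the construction script do nothing, so playback starts only when an event is called.
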(event `self.ReceiveBeginPlay`)

(event `Play`
  (bind (_direction _newtrack_0 _newtrack_1) (`Timeline|Timeline_0` :`NewTime` (stale `SetNewTime` NewTime) :!label _label)
    (:`Update`
      (`KismetSystemLibrary.PrintString` (`KismetStringLibrary.Concat_StrStr` (`|GetEnumeratorNameAsString` _direction) (`KismetStringLibrary.Conv_DoubleToString` _newtrack_0) (`KismetStringLibrary.Conv_VectorToString` _newtrack_1))))
    (:`Finished`
      (`KismetSystemLibrary.PrintString` "Finished"))))

(event `PlayFromStart`
  (goto _label :!via `PlayFromStart`))

(event `Stop`
  (goto _label :!via `Stop`))

(event `Reverse`
  (goto _label :!via `Reverse`))

(event `ReverseFromEnd`
  (goto _label :!via `ReverseFromEnd`))

(event `SetNewTime`
  (params (NewTime :type "Float (double-precision)"))
  (goto _label :!via `SetNewTime`))

(fn `UserConstructionScript`)